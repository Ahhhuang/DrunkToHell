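; Fan actor that blows the player character along the up vector of its Cone1 component.
; Box overlap begin and end events toggle an inside flag without checking which actor overlapped.
; While the flag is set, Tick casts player 0's character to ThirdPersonCharacter and sets its movement velocity to the controlled pawn's velocity plus that direction scaled by WindStrength.
; The push accumulates every frame without delta-time scaling.
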(event `self.Box.OnComponentBeginOverlap`
  (params (OverlappedComponent :type "PrimitiveComponent Object Reference") (OtherActor :type "Actor Object Reference") (OtherComp :type "PrimitiveComponent Object Reference") (OtherBodyIndex :type Integer) (bFromSweep :type Boolean) (SweepResult :type "HitResult Structure (by ref)"))
  (set `self.IsInsideBox?` true))

(event `self.ReceiveTick`
  (params (DeltaSeconds :type "Float (single-precision)"))
  (if (`self.IsInsideBox?`)
    (bind _asthird_person_character (cast `/Game/ThirdPersonBP/Blueprints/ThirdPersonCharacter` (`GameplayStatics.GetPlayerCharacter` 0)))
    (set `MovementComponent.Velocity` (+ (`self.GetVelocity` (`Controller.K2_GetPawn` (`GameplayStatics.GetPlayerController` 0))) (* (* (`SceneComponent.GetUpVector` (`self.Cone1`)) 1) (`self.WindStrength`))) (`Character.CharacterMovement` _asthird_person_character))))

(event `self.Box.OnComponentEndOverlap`
  (params (OverlappedComponent :type "PrimitiveComponent Object Reference") (OtherActor :type "Actor Object Reference") (OtherComp :type "PrimitiveComponent Object Reference") (OtherBodyIndex :type Integer))
  (set `self.IsInsideBox?` false))

(fn `UserConstructionScript`)