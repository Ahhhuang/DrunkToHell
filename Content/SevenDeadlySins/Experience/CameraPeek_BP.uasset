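; Peek spot actor that lets the player press E inside its trigger box to view through its camera, with movement locked and hint messages.
; The camera nudges with the player's turn and look input within a range of its start position, always facing a target point.
; The first peek plays a movie, reveals one set of actors and destroys another.
; Exiting is blocked until the movie's time reads zero.
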(event `self.ReceiveTick`
  (params (DeltaSeconds :type "Float (single-precision)"))
  (bind _returnvalue (`GameplayStatics.GetPlayerController` 0))
  (bind _cameramovscale (`self.CameraMovScale`))
  (bind _camera (`self.Camera`))
  (bind _returnvalue_2 (`SceneComponent.K2_GetComponentLocation` _camera))
  (bind _asthird_person_character (cast `/Game/ThirdPersonBP/Blueprints/ThirdPersonCharacter` (`GameplayStatics.GetPlayerCharacter` 0)))
  (bind _returnvalue_3 (`KismetMathLibrary.MakeVector` (.x (`SceneComponent.K2_GetComponentLocation` (`self.Camera`))) (+ (.y (`SceneComponent.K2_GetComponentLocation` (`self.Camera`))) (* (`/Game/ThirdPersonBP/Blueprints/ThirdPersonCharacter.TurnVar` _asthird_person_character) _cameramovscale)) (+ (.z (`SceneComponent.K2_GetComponentLocation` (`self.Camera`))) (* _cameramovscale (`/Game/ThirdPersonBP/Blueprints/ThirdPersonCharacter.LookUpVar` _asthird_person_character)))))
  (if (<= (`KismetMathLibrary.Vector_Distance` (`self.CameraInitPos`) _returnvalue_3) (`self.CameraRange`))
    (set `self.CameraTarPos` _returnvalue_3)
    (else
      (set `self.CameraTarPos` _returnvalue_2)))
  (`SceneComponent.K2_SetWorldLocation` _camera (`KismetMathLibrary.VLerp` _returnvalue_2 (`self.CameraTarPos`) 0.2) false false)
  (`SceneComponent.K2_SetWorldRotation` (`self.Camera`) (`KismetMathLibrary.FindLookAtRotation` (`SceneComponent.K2_GetComponentLocation` (`self.Camera`)) (`SceneComponent.K2_GetComponentLocation` (`self.TargetPoint`))) false false)
  (if (and (`self.IsInside?`) (`self.CanExit?`))
    (if (`PlayerController.WasInputKeyJustPressed` (`GameplayStatics.GetPlayerController` 0) "E")
      (if (`self.IsPeeking?`)
        (bind _asthird_person_character_2 (cast `/Game/ThirdPersonBP/Blueprints/ThirdPersonCharacter` (`GameplayStatics.GetPlayerCharacter` 0)))
        (`PlayerController.SetViewTargetWithBlend` _returnvalue _asthird_person_character_2 0.4 "VTBlend_EaseOut" 0.3 false)
        (set `self.IsPeeking?` false)
        (bind _asthird_person_character_3 (cast `/Game/ThirdPersonBP/Blueprints/ThirdPersonCharacter` (`GameplayStatics.GetPlayerCharacter` 0)))
        (set `/Game/ThirdPersonBP/Blueprints/ThirdPersonCharacter.HintMessage` "Press \"E\" to Peek" _asthird_person_character_3)
        (set `/Game/ThirdPersonBP/Blueprints/ThirdPersonCharacter.CanMove?` true _asthird_person_character_3)
        (`SceneComponent.SetHiddenInGame` (`self.MovieHolder`) true false)
        (else
          (`PlayerController.SetViewTargetWithBlend` _returnvalue self 0.4 "VTBlend_EaseOut" 0.3 false)
          (set `self.IsPeeking?` true)
          (bind _asthird_person_character_4 (cast `/Game/ThirdPersonBP/Blueprints/ThirdPersonCharacter` (`GameplayStatics.GetPlayerCharacter` 0)))
          (set `/Game/ThirdPersonBP/Blueprints/ThirdPersonCharacter.CanMove?` false _asthird_person_character_4)
          (if (`self.MediaPlayerHasPlayed?`)
            (set `/Game/ThirdPersonBP/Blueprints/ThirdPersonCharacter.HintMessage` "Press \"E\" to Exit" _asthird_person_character_4)
            (else
              (set `/Game/ThirdPersonBP/Blueprints/ThirdPersonCharacter.HintMessage` "" _asthird_person_character_4)
              (`SceneComponent.SetHiddenInGame` (`self.MovieHolder`) false false)
              (bind _output_get (set `self.MediaPlayer` (`self.MediaPlayer`)))
              (`MediaPlayer.Play` _output_get)
              (`KismetSystemLibrary.Delay` 0.4)
              (`self.EnableActors` true (`self.ActorsShouldOpen`))
              (`self.EnableActors` false (`self.ActorsShouldClose`) true)
              (set `self.CanExit?` false))))))
    (elif (not (`self.CanExit?`))
      (if (== (`MediaPlayer.GetTime` (`self.MediaPlayer`)) (`KismetMathLibrary.TimespanZeroValue`))
        (`SceneComponent.SetHiddenInGame` (`self.MovieHolder`) true false)
        (set `self.CanExit?` true)
        (set `self.MediaPlayerHasPlayed?` true)
        (bind _asthird_person_character_5 (cast `/Game/ThirdPersonBP/Blueprints/ThirdPersonCharacter` (`GameplayStatics.GetPlayerCharacter` 0)))
        (set `/Game/ThirdPersonBP/Blueprints/ThirdPersonCharacter.HintMessage` "Press \"E\" to Exit" _asthird_person_character_5)))))

(event `self.TriggerBox.OnComponentBeginOverlap`
  (params (OverlappedComponent :type "PrimitiveComponent Object Reference") (OtherActor :type "Actor Object Reference") (OtherComp :type "PrimitiveComponent Object Reference") (OtherBodyIndex :type Integer) (bFromSweep :type Boolean) (SweepResult :type "HitResult Structure (by ref)"))
  (bind _asthird_person_character (cast `/Game/ThirdPersonBP/Blueprints/ThirdPersonCharacter` OtherActor))
  (set `/Game/ThirdPersonBP/Blueprints/ThirdPersonCharacter.HintMessage` "Press \"E\" to Peek" _asthird_person_character)
  (set `self.IsInside?` true)
  (bind _output_get (set `self.MediaPlayer` (`self.MediaPlayer`)))
  (`MediaPlayer.OpenSource` _output_get (`self.MediaSource`))
  (`SceneComponent.SetHiddenInGame` (`self.MovieHolder`) true false))

(event `self.TriggerBox.OnComponentEndOverlap`
  (params (OverlappedComponent :type "PrimitiveComponent Object Reference") (OtherActor :type "Actor Object Reference") (OtherComp :type "PrimitiveComponent Object Reference") (OtherBodyIndex :type Integer))
  (bind _asthird_person_character (cast `/Game/ThirdPersonBP/Blueprints/ThirdPersonCharacter` OtherActor))
  (set `/Game/ThirdPersonBP/Blueprints/ThirdPersonCharacter.HintMessage` "" _asthird_person_character)
  (set `self.IsInside?` false))

(event `self.ReceiveBeginPlay`
  (set `self.CameraInitPos` (`SceneComponent.K2_GetComponentLocation` (`self.Camera`))))

(fn `EnableActors`
  (params (SetEnable :type Boolean) (ActorArray :type "Array of Actor Object Reference") (Destroy :type Boolean))
  (if Destroy
    (for _array_element ActorArray
      (`self.K2_DestroyActor` _array_element))
    (else
      (for _array_element_2 ActorArray
        (`SceneComponent.SetVisibility` (`Actor.RootComponent` _array_element_2) SetEnable true)
        (`self.SetActorHiddenInGame` _array_element_2 (not SetEnable))
        (`self.SetActorEnableCollision` _array_element_2 SetEnable)
        (`self.SetActorTickEnabled` _array_element_2 SetEnable)))))

(fn `UserConstructionScript`)