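; SoundClick_BP is a trigger Blueprint that plays love music and silences it while something overlaps its box.
; The LoveMusicSoundCue audio component starts on BeginPlay.
; Box begin overlap pauses the audio if it is playing, and end overlap resumes it if paused.
; The overlap events do not filter by actor, so any overlapping object toggles the music.
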(event `self.Box.OnComponentBeginOverlap`
  (params (OverlappedComponent :type "PrimitiveComponent Object Reference") (OtherActor :type "Actor Object Reference") (OtherComp :type "PrimitiveComponent Object Reference") (OtherBodyIndex :type Integer) (bFromSweep :type Boolean) (SweepResult :type "HitResult Structure (by ref)"))
  (bind _lovemusicsoundcue (`self.LoveMusicSoundCue`))
  (if (== (enumliteral `EAudioComponentPlayState` "Playing") (`AudioComponent.GetPlayState` _lovemusicsoundcue))
    (`AudioComponent.SetPaused` _lovemusicsoundcue true)))

(event `self.Box.OnComponentEndOverlap`
  (params (OverlappedComponent :type "PrimitiveComponent Object Reference") (OtherActor :type "Actor Object Reference") (OtherComp :type "PrimitiveComponent Object Reference") (OtherBodyIndex :type Integer))
  (bind _lovemusicsoundcue (`self.LoveMusicSoundCue`))
  (if (== (enumliteral `EAudioComponentPlayState` "Paused") (`AudioComponent.GetPlayState` _lovemusicsoundcue))
    (`AudioComponent.SetPaused` _lovemusicsoundcue false)))

(event `self.ReceiveBeginPlay`
  (`AudioComponent.Play` (`self.LoveMusicSoundCue`) 0.0))

(fn `UserConstructionScript`)